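; BP_EnemyController is the enemy AI controller, running BT_EnemyBehavior and freezing the enemy while it is in light.
; Each tick it writes the first AIPerception stimulus result for the player to the HasSeenPlayer blackboard key.
; It then deactivates or reactivates CharacterMovement based on InLight, which is not set in this graph.
; The controlled enemy reference comes from GetActorOfClass rather than the possessed pawn.
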(event Custom|CheckLight
  (bind _enemyrefrence (Variables|Default|GetEnemyRefrence))
  (bind _charactermovement (Variables|/Script/Engine.Character|GetCharacterMovement _enemyrefrence))
  ;[0 0 0] Freezes enemy if in light path
  (if (Variables|Default|GetInLight)
    (Components|Activation|Deactivate _charactermovement)
    (else
      (Components|Activation|Activate _charactermovement false))))

(event EventBeginPlay
  ;[0 0 0] Runs enemy behavior
  (AI|RunBehaviorTree "/Game/Blueprint/Enemy/BT_EnemyBehavior.BT_EnemyBehavior")
  (bind _returnvalue (Actor|GetActorOfClass "/Game/Blueprint/Enemy/BP_EnemyCharacter.BP_EnemyCharacter_C"))
  (Variables|Default|SetEnemyRefrence _returnvalue))

(event EventTick
  (params (DeltaSeconds :type Float%20%28single-precision%29))
  ;[0 0 0] Looks for player and switches bool if seen
  (bind _info (Class|AIPerceptionComponent|GetActorsPerception (Variables|Default|GetAIPerception) (Game|Player|GetPlayerPawn 0)))
  (AI|Components|Blackboard|SetValueasBool (AI|GetBlackboard (AI|GetAIController self)) (Utilities|Name|MakeLiteralName "HasSeenPlayer") (.bSuccessfullySensed (Utilities|Struct|BreakAIStimulus (Utilities|Array|Get(acopy) (.lastsensedstimuli _info)))))
  ;[0 0 0] Runs check light
  (CallFunction|CheckLight))

(fn ConstructionScript)