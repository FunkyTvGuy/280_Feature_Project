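; BP_PlayerCharacter is the player-controlled character, which moves, aims a flashlight and dies on contact with an enemy.
; BeginPlay adds the Enhanced Input mapping context and finds the level's BP_FlashLight actor.
; Movement input follows control rotation, while rotate input drives the flashlight's MoveFlashlight and toggles its IsMovingLight flag.
; Overlapping a BP_EnemyCharacter calls Kill on BP_PlayerController, which is fetched as player 0.
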(event Input|EnhancedActionEvents|EnhancedInputActionIA_Movement
  (params (ActionValue :type Vector%202D%20Structure) (ElapsedSeconds :type Float%20%28double-precision%29) (TriggeredSeconds :type Float%20%28double-precision%29) (InputAction :type Input%20Action%20Object%20Reference :default "/Game/Blueprint/Inputs/IA_Movement.IA_Movement"))
  (bind _returnvalue (Pawn|GetControlRotation :!class /Script/Engine.Pawn))
  ;[0 0 0] Enhanced move input
  (Pawn|Input|AddMovementInput (Math|Vector|GetRightVector (Math|Rotator|MakeRotator (.roll _returnvalue) 0.0 (.yaw _returnvalue))) (.y ActionValue) false)
  (Pawn|Input|AddMovementInput (Math|Vector|GetForwardVector (Math|Rotator|MakeRotator 0.0 0.0 (.yaw (Pawn|GetControlRotation :!class /Script/Engine.Pawn)))) (.x ActionValue) false))

(event Input|EnhancedActionEvents|EnhancedInputActionIA_FlashlightRotate
  (params (ActionValue :type Vector%202D%20Structure) (ElapsedSeconds :type Float%20%28double-precision%29) (TriggeredSeconds :type Float%20%28double-precision%29) (InputAction :type Input%20Action%20Object%20Reference :default "/Game/Blueprint/Inputs/IA_FlashlightRotate.IA_FlashlightRotate"))
  (bind _flashlight (Variables|Default|GetFlashlight))
  ;[0 0 0] Checks if flashlight should be moved
  (:Triggered
    (Default|MoveFlashlight _flashlight (.x ActionValue) (.y ActionValue))
    (Variables|/Game/Blueprint/BP_FlashLight.BP_FlashLight_C|SetIsMovingLight _flashlight true))
  (:Completed
    (Variables|/Game/Blueprint/BP_FlashLight.BP_FlashLight_C|SetIsMovingLight _flashlight false)))

(event EventBeginPlay
  ;[0 0 0] Set up player input mapping conntext
  (bind _asbp_player_controller (Utilities|Casting|CastToBP_PlayerController (Game|GetPlayerController 0)))
  (Utilities|IsValid (PlayerController|LocalPlayerSubsystems|GetEnhancedInputLocalPlayerSubsystem _asbp_player_controller)
    (:Is%20Valid
      (Input|AddMappingContext (PlayerController|LocalPlayerSubsystems|GetEnhancedInputLocalPlayerSubsystem _asbp_player_controller) "/Game/Blueprint/Inputs/IMC_PlayerController.IMC_PlayerController" 0 "(bIgnoreAllPressedKeysUntilRelease=True,bForceImmediately=False,bNotifyUserSettings=False)")
      ;[0 0 0] Get refrence to flashlight
      (bind _returnvalue (Actor|GetActorOfClass "/Game/Blueprint/BP_FlashLight.BP_FlashLight_C"))
      (Variables|Default|SetFlashlight _returnvalue))))

(event Collision|EventActorBeginOverlap
  (params (OtherActor :type Actor%20Object%20Reference))
  ;[0 0 0] Overlap with enemy
  (Utilities|Casting|CastToBP_EnemyCharacter OtherActor)
  (bind _asbp_player_controller (Utilities|Casting|CastToBP_PlayerController (Game|GetPlayerController 0)))
  (Default|Kill _asbp_player_controller))

(fn ConstructionScript)