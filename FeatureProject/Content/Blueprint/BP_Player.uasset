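; BP_Player is a player Blueprint intended to handle Enhanced Input movement and death on enemy contact.
; BeginPlay, the IA_Movement action and the Hit event are all empty, with their logic left in disconnected nodes that never run.
; Those nodes would add the IMC_PlayerController mapping context, move along the actor's forward and right vectors, and call Kill on BP_PlayerController when hitting a BP_EnemyCharacter.
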(event Input|EnhancedActionEvents|EnhancedInputActionIA_Movement
  (params (ActionValue :type Vector%202D%20Structure) (ElapsedSeconds :type Float%20%28double-precision%29) (TriggeredSeconds :type Float%20%28double-precision%29) (InputAction :type Input%20Action%20Object%20Reference :default "/Game/Blueprint/Inputs/IA_Movement.IA_Movement"))
  ;[0 0 0] Enhanced move input
)

(event EventBeginPlay
  ;[0 0 0] Set up player input mapping conntext
)

(event Collision|EventHit
  (params (MyComp :type Primitive%20Component%20Object%20Reference) (Other :type Actor%20Object%20Reference) (OtherComp :type Primitive%20Component%20Object%20Reference) (bSelfMoved :type Boolean) (HitLocation :type Vector :default "0, 0, 0") (HitNormal :type Vector :default "0, 0, 0") (NormalImpulse :type Vector :default "0, 0, 0") (Hit :type Hit%20Result%20Structure%20%28by%20ref%29))
  ;[0 0 0] Overlap with enemy
)

(fn ConstructionScript)